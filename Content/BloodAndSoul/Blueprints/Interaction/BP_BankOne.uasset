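; Interactable bank that opens a banking UI when the player interacts with it.
; On BeginPlay it binds range, interact and disengage events to handler functions, with range changes only printing messages.
; Interacting disables the interactor's input, creates WBP_Bank with a reference back to itself and shows the cursor; disengaging reverses this.
; OpenWidget duplicates the interact logic minus the greeting and is not called within this Blueprint.
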(event `self.ReceiveBeginPlay`
  (add `self.OnInteractorMovedIntoRange` (delegate `OnInteractorMovedIntoRangeEvent`))
  (add `self.OnInteractorMovedOutOfRange` (delegate `OnInteractorMovedOutOfRangEvent`))
  (add `self.OnInteraction` (delegate `OnInteractionEvent`))
  (add `self.OnDisengage` (delegate `OnDisengageEvent`)))

(event `OnInteractorMovedIntoRangeEvent`
  (`self.InteractorMovedIntoRange`))

(event `OnInteractorMovedOutOfRangEvent`
  (`self.InteractorMovedOutOfRange`))

(event `OnInteractionEvent`
  (`self.InteractCallback`))

(event `OnDisengageEvent`
  (`self.DisengageCallback`))

(fn `CloseWidget`
  (bind _returnvalue (`GameplayStatics.GetPlayerController` 0))
  (`Widget.RemoveFromParent` (`self.BankWidget`))
  (set `PlayerController.bShowMouseCursor` false _returnvalue)
  (`self.EnableInput` (`self.GetInteractor`) _returnvalue))

(fn `DisengageCallback`
  (`self.CloseWidget`))

(fn `InteractCallback`
  (bind _returnvalue (`GameplayStatics.GetPlayerController` 0))
  (`KismetSystemLibrary.PrintString` "Hello Sir, we are the best bank all aroun, would you like to deposit something!")
  (`self.DisableInput` (`self.GetInteractor`) _returnvalue)
  (bind _returnvalue_2 (`|CreateWidget` "/Game/BloodAndSoul/Graphics/UI/Bank/WBP_Bank.WBP_Bank_C" _returnvalue))
  (bind _output_get (set `self.BankWidget` _returnvalue_2))
  (`/Game/BloodAndSoul/Graphics/UI/Bank/WBP_Bank.SetBankInteractable` _output_get self)
  (`UserWidget.AddToViewport` (`self.BankWidget`) 0)
  (set `PlayerController.bShowMouseCursor` true (`GameplayStatics.GetPlayerController` 0)))

(fn `InteractorMovedIntoRange`
  (`KismetSystemLibrary.PrintString` "Press F to interact"))

(fn `InteractorMovedOutOfRange`
  (`KismetSystemLibrary.PrintString` "Ah, the player moved out of the interaction zone..."))

(fn `OpenWidget`
  (bind _returnvalue (`GameplayStatics.GetPlayerController` 0))
  (`self.DisableInput` (`self.GetInteractor`) _returnvalue)
  (bind _returnvalue_2 (`|CreateWidget` "/Game/BloodAndSoul/Graphics/UI/Bank/WBP_Bank.WBP_Bank_C" _returnvalue))
  (bind _output_get (set `self.BankWidget` _returnvalue_2))
  (set `/Game/BloodAndSoul/Graphics/UI/Bank/WBP_Bank.BankInteractable` self _output_get)
  (`UserWidget.AddToViewport` (`self.BankWidget`) 0)
  (set `PlayerController.bShowMouseCursor` true (`GameplayStatics.GetPlayerController` 0)))

(fn `UserConstructionScript`)